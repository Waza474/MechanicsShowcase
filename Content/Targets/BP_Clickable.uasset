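; BP_Clickable makes its owning actor selectable as the player's target by mouse click, apparently as an actor component.
; On BeginPlay it binds to the owner's OnClicked event.
; A click prints the actor's name, passes the owner to BP_NewPlayerController's SetNewTarget, then binds ClearTarget to that controller's TargetChanged event.
; ClearTarget is an empty stub, so a target change currently triggers no response here.
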(event `self.ReceiveBeginPlay`
  (add `Actor.OnClicked` (`self.GetOwner`) (delegate `OnMouseClick`)))

(event `OnMouseClick`
  (params (TouchedActor :type "Actor Object Reference") (ButtonPressed :type "Key Structure" :default "None"))
  (`KismetSystemLibrary.PrintString` (`KismetSystemLibrary.GetDisplayName` TouchedActor))
  (bind _asbp_new_player_controller (cast `/Game/ThirdPerson/Blueprints/BP_NewPlayerController` (`GameplayStatics.GetPlayerController` 0)))
  (`/Game/ThirdPerson/Blueprints/BP_NewPlayerController.Set New Target` _asbp_new_player_controller (`self.GetOwner`))
  (add `/Game/ThirdPerson/Blueprints/BP_NewPlayerController.Target Changed` _asbp_new_player_controller (delegate `Clear Target`)))

(event `Clear Target`)